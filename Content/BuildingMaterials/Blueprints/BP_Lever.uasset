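; BP_Lever is a VR lever that stores the motion controller on Grab and clears it when that controller releases.
; Tick checks the stored controller but does nothing with it, as the handle rotation logic is disconnected and never runs.
; That unused logic converts the controller position into handle space, derives a look-at pitch and adds it to the handle's pitch, clamped to a quarter turn.
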(event EventTick
  (params (DeltaSeconds :type Float%20%28single-precision%29))
  (bind _motion_controller (Variables|Default|GetMotion%20Controller)
    (:then)
    (:else)))

(event EventRelease
  (params (MotionController :type Motion%20Controller%20Component%20Object%20Reference))
  (if (== (Variables|Default|GetMotion%20Controller) MotionController)
    (Variables|Default|SetMotion%20Controller 0)))

(event EventGrab
  (params (MotionController :type Motion%20Controller%20Component%20Object%20Reference))
  (Variables|Default|SetMotion%20Controller MotionController))

(fn ConstructionScript)